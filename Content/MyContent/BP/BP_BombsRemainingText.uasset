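; BP_BombsRemainingText is a text display that shows how many bombs remain in the game.
; On BeginPlay it casts the game instance to GI_Game, resets BombsRemaining to BombsNeeded and writes that count into TextToChange.
; It then binds UpdateBombText to the game instance's UpdateBombsText dispatcher, so the number refreshes on each broadcast instead of polling every tick.
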(event Custom|UpdateBombText
  (Rendering|Components|TextRender|SetText (Variables|Default|GetTextToChange) (Utilities|Text|ToText(Integer) (Variables|/Game/MyContent/Game/GI_Game.GI_Game_C|GetbombsRemaining (Variables|Default|GetAs%20GI%20Game)))))

(event EventBeginPlay
  (bind _asgi_game (Utilities|Casting|CastToGI_Game (Game|GetGameInstance)))
  (bind _output_get (Variables|Default|SetAs%20GI%20Game _asgi_game))
  (Variables|/Game/MyContent/Game/GI_Game.GI_Game_C|SetbombsRemaining _output_get (Variables|/Game/MyContent/Game/GI_Game.GI_Game_C|GetbombsNeeded _output_get))
  (CallFunction|UpdateBombText)
  (EventDispatchers|BindEventtoUpdateBombsText (Variables|Default|GetAs%20GI%20Game) (delegate Custom|UpdateBombText)))

(fn ConstructionScript)