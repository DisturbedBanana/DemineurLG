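; BP_PlayerPawn is the player pawn, with a camera that shifts toward the bomb's position when the game is lost.
; LostTheGame receives the bomb position and starts a looping timer that fires GoToBomb, with nothing here stopping it.
; GoToBomb sets the camera's world location by interpolating each axis from DefaultSceneRoot's location, not the camera's, toward the bomb's X and Y and a fixed height.
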(event Custom|LostTheGame
  (params (BombPos :type Vector))
  (Utilities|Time|SetTimerbyEvent (delegate Custom|GoToBomb) 0.01 true))

(event Custom|GoToBomb
  (bind _returnvalue (Utilities|Time|GetWorldDeltaSeconds))
  (bind _self self)
  (bind _defaultsceneroot (Variables|Default|GetDefaultSceneRoot _self))
  (bind _returnvalue_2 (Transformation|GetWorldLocation _defaultsceneroot))
  (Transformation|SetWorldLocation (Variables|Default|GetCamera) (Math|Vector|MakeVector (Math|Interpolation|FInterpTo (.x _returnvalue_2) (.x (stale Custom|LostTheGame BombPos)) _returnvalue 2.0) (Math|Interpolation|FInterpTo (.y _returnvalue_2) (.y (stale Custom|LostTheGame BombPos)) _returnvalue 2.0) (Math|Interpolation|FInterpTo (.z _returnvalue_2) 5e+01 _returnvalue 2.0)) false false))

(fn ConstructionScript)