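; Minesweeper-style playground actor that builds the tile board and places mines at BeginPlay.
; It scales its plane mesh by the GI_Game difficulty, then uses the scaled bounds to spawn the game instance's tile count in wrapped rows.
; Repeated passes over the tiles turn non-mines into mines at 1-in-8 odds via three chained RandomBools until the required count is reached, then every tile is initialized.
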(event Custom|SpawnTiles
  ;[1 1 1] Set first spawn position
  (Variables|Default|SetposX (Variables|Default|GetxMin))
  (Variables|Default|SetposY (+ (Variables|Default|GetyMin) (Variables|Default|GetyOffset)))
  ;[1 1 1] Spawn all tiles
  (for _index (range 0 (- (Variables|/Game/MyContent/Game/GI_Game.GI_Game_C|GetnbOfTiles (Variables|Default|GetAs%20GI%20Game)) 1))
    (if (>= (+ (+ (Variables|Default|GetposX) 3e+01) (Variables|Default|GetxOffset)) (Variables|Default|GetxMax))
      ;[1 1 1] Set spawn position 1 row lower and all the way back to the left
      (Variables|Default|SetposY (+ (Variables|Default|GetposY) (Variables|Default|GetyOffset)))
      (Variables|Default|SetposX (+ (Variables|Default|GetxMin) (Variables|Default|GetxOffset)))
      (else
        ;[1 1 1] Set spawn position further right
        (Variables|Default|SetposX (+ (Variables|Default|GetposX) (Variables|Default|GetxOffset)))))
    (bind _returnvalue (Game|SpawnActorfromClass "/Game/MyContent/BP/BP_Tile.BP_Tile_C" (Math|Conversions|ToTransform(Vector) (Math|Vector|MakeVector (Variables|Default|GetposX) (Variables|Default|GetposY) 0.0)) "Undefined" 0 0 0))
    (Utilities|Array|Add (Variables|Default|GetTileList) _returnvalue))
  (CallFunction|SetBombs))

(event Custom|GetBounds
  (bind _staticmesh (Variables|Default|GetStaticMesh))
  (bind (_min _max) (Components|StaticMesh|GetLocalBounds _staticmesh))
  (bind _returnvalue (Transformation|GetWorldScale _staticmesh))
  (bind _returnvalue_2 (* _max _returnvalue))
  (bind _returnvalue_3 (* _min _returnvalue))
  (bind (_x _y) (Math|Vector|BreakVector _returnvalue_2))
  (bind (_x_2 _y_2) (Math|Vector|BreakVector _returnvalue_3))
  ;[1 1 1] Get the bounds of the gameplay planen used to Spawn the tiles on top of it
  (Variables|Default|SetxMin _x_2)
  (Variables|Default|SetxMax _x)
  (Variables|Default|SetyMin _y_2)
  (Variables|Default|SetyMax _y)
  (CallFunction|SpawnTiles))

(event Custom|SetBombs
  (bind _as_gi_game (Variables|Default|GetAs%20GI%20Game))
  (bind _as_gi_game_2 (Variables|Default|GetAs%20GI%20Game))
  ;[1 1 1] While there is less bombs than needed
  (while (< (Variables|/Game/MyContent/Game/GI_Game.GI_Game_C|GetbombsPresent _as_gi_game) (Variables|/Game/MyContent/Game/GI_Game.GI_Game_C|GetbombsNeeded _as_gi_game))
    (bind _array_element (Utilities|Array|ForEachLoopwithBreak (Variables|Default|GetTileList) :!label _label)
      (:LoopBody
        ;[1 1 1] Stop foreach to prevent getting too much bombs
        (if (< (Variables|/Game/MyContent/Game/GI_Game.GI_Game_C|GetbombsPresent _as_gi_game_2) (Variables|/Game/MyContent/Game/GI_Game.GI_Game_C|GetbombsNeeded _as_gi_game_2))
          (bind _output_get (Variables|Default|SetIteratedTile _array_element))
          ;[1 1 1] If this tile already isn't a bomb
          (if (not (Variables|/Game/MyContent/BP/BP_Tile.BP_Tile_C|GetisMine _output_get))
            ;[1 1 1] 1 of 8 to succeed ( random int was breaking loop :(     )
            (if (Math|Random|RandomBool)
              (if (Math|Random|RandomBool)
                (if (Math|Random|RandomBool)
                  ;[1 1 1] Tile becomes a bomb and increment number of bombs
                  (Variables|/Game/MyContent/BP/BP_Tile.BP_Tile_C|SetisMine (Variables|Default|GetIteratedTile) true)
                  (bind _result (Math|Integer|IncrementInt (Variables|/Game/MyContent/Game/GI_Game.GI_Game_C|GetbombsPresent (Variables|Default|GetAs%20GI%20Game)))
                    (:%20%20
                      (Variables|/Game/MyContent/Game/GI_Game.GI_Game_C|SetbombsPresent (Variables|Default|GetAs%20GI%20Game) _result)))))))
          (else
            (goto _label Break))))))
  (for _array_element_2 (Variables|Default|GetTileList)
    (Default|InitializeTile _array_element_2)))

(event EventBeginPlay
  (bind _staticmesh (Variables|Default|GetStaticMesh))
  (bind _asgi_game (Utilities|Casting|CastToGI_Game (Game|GetGameInstance)))
  (bind _output_get (Variables|Default|SetAs%20GI%20Game _asgi_game))
  ;[1 1 1] Set Plane size depending on difficulty
  (switch int (Variables|/Game/MyContent/Game/GI_Game.GI_Game_C|Getdifficulty _output_get)
    (:0
      (Transformation|SetWorldScale3D _staticmesh (Math|Vector|MakeVector 4.4 4.4 0.0)))
    (:1
      (Transformation|SetWorldScale3D _staticmesh (Math|Vector|MakeVector 3.2 3.6 0.0)))
    (:2
      (Transformation|SetWorldScale3D _staticmesh (Math|Vector|MakeVector 6.8 6.8 0.0)))
    (:3
      (Transformation|SetWorldScale3D _staticmesh (Math|Vector|MakeVector 6.8 13.0 0.0))))
  (Transformation|SetWorldLocation (Variables|Default|GetStaticMesh) "0, 0, 0" false false)
  (CallFunction|GetBounds))

(fn ConstructionScript)