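; Actor component that picks the Minesweeper-style tile under the player's mouse cursor and updates it.
; CastLineTrace runs a complex Visibility trace from the cursor, casts the hit actor to BP_Tile, stores it and calls its UpdateTile.
; It then prints debug messages showing the tile's adjacent bomb count and whether its left and right neighbor references are valid.
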(event Custom|CastLineTrace
  (bind _asbp_tile (Utilities|Casting|CastToBP_Tile (.HitActor (Collision|BreakHitResult (.HitResult (Game|Player|GetHitResultUnderCursorbyChannel (Game|GetPlayerController 0) "TraceTypeQuery1" true))))))
  (Variables|Default|SetAs%20BP%20Tile _asbp_tile)
  (Default|UpdateTile (Variables|Default|GetAs%20BP%20Tile))
  (Development|PrintString (Utilities|String|ToString(Integer) (Variables|/Game/MyContent/BP/BP_Tile.BP_Tile_C|GetnbOfAdjacentBombs (Variables|Default|GetAs%20BP%20Tile))))
  (Variables|/Game/MyContent/BP/BP_Tile.BP_Tile_C|GetTileOnTheRight (Variables|Default|GetAs%20BP%20Tile)
    (:then
      (Development|PrintString "right is valid" true true "(R=1.000000,G=0.000000,B=0.000000,A=1.000000)" 1e+01))
    (:else
      (Development|PrintString "right isnt valid" true true "(R=1.000000,G=0.000000,B=0.000000,A=1.000000)" 1e+01)))
  (Variables|/Game/MyContent/BP/BP_Tile.BP_Tile_C|GetTileOnTheLeft (Variables|Default|GetAs%20BP%20Tile)
    (:then
      (Development|PrintString "left is valid" true true "(R=1.000000,G=0.000000,B=0.000000,A=1.000000)" 1e+01))
    (:else
      (Development|PrintString "left isnt valid" true true "(R=1.000000,G=0.000000,B=0.000000,A=1.000000)" 1e+01))))